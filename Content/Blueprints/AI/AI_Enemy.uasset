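; AI_Enemy is an enemy AI controller that runs the BT_Enemy behavior tree and feeds it player awareness through the blackboard.
; On BeginPlay it starts the tree and sets an initial enemy behavior type.
; AI Perception updates for BP_Player record whether the player is sensed.
; Tick sets KnowAboutPlayer when the player is within a fixed distance or currently sensed, so proximity alone triggers awareness.
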(event `self.ReceiveBeginPlay`
  (`self.RunBehaviorTree` "/Game/Blueprints/AI/BT_Enemy.BT_Enemy")
  (`self.Set Behavior` "NewEnumerator1"))

(event `self.ReceiveTick`
  (params (DeltaSeconds :type "Float (single-precision)"))
  (`self.Set Know About Player` (or (<= (`self.GetDistanceTo` (`self.K2_GetPawn`) (`GameplayStatics.GetPlayerPawn` 0)) 1000.0) (`self.CanSeePlayer_Sense`))))

(event `self.AIPerception.OnTargetPerceptionUpdated`
  (params (Actor :type "Actor Object Reference") (Stimulus :type "AIStimulus Structure"))
  (cast `/Game/Blueprints/BP_Player` Actor)
  (bind _output_get (set `self.CanSeePlayer_Sense` (`.bSuccessfullySensed` (break `AIStimulus` Stimulus))))
  (`BlackboardComponent.SetValueAsBool` (`AIBlueprintHelperLibrary.GetBlackboard` null) "CanSeePlayer_Sense" _output_get))

(fn `Set Behavior`
  (params (Enum :type "/Game/Blueprints/AI/E_EnemyBehaviorType Enum" :default "NewEnumerator0"))
  (`BlackboardComponent.SetValueAsEnum` (`self.Blackboard`) "EnemyBehaviorType" (enumliteral `/Game/Blueprints/AI/E_EnemyBehaviorType` Enum)))

(fn `Set Know About Player`
  (params (BoolValue :type Boolean))
  (`BlackboardComponent.SetValueAsBool` (`AIBlueprintHelperLibrary.GetBlackboard` null) "KnowAboutPlayer" BoolValue))

(fn `UserConstructionScript`)