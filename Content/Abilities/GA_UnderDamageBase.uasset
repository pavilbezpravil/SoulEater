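; GA_UnderDamageBase is a Gameplay Ability that plays a hit-impact montage on the avatar, apparently as a base for damage-reaction abilities.
; On activation it commits, casts the avatar to Character and plays ImpactMontage through PlayMontageAndWait.
; The ability ends on montage blend-out, interruption or cancellation, or immediately if the commit or cast fails.
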(event `self.K2_ActivateAbility`
  (`parent.K2_ActivateAbility`)
  (bind _returnvalue (`self.K2_CommitAbility`))
  (if _returnvalue
    (cast `Character` (`self.GetAvatarActorFromActorInfo`)
      (:`then`
        (`AbilityTask_PlayMontageAndWait.CreatePlayMontageAndWaitProxy` "None" (`self.Impact Montage`)
          (:`OnBlendOut`
            _)
          (:`OnInterrupted`
            _)
          (:`OnCancelled`
            _))
        (`self.K2_EndAbility`))
      (:`CastFailed`
        (`self.K2_EndAbility`)))
    (else
      (`self.K2_EndAbility`))))