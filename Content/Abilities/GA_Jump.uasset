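; GA_Jump is a gameplay ability that makes the avatar character jump.
; On activation it commits the ability, then calls Jump on the avatar's SE character base if that reference is valid.
; The ability then ends immediately; a disconnected branch that would apply a GE_Jump effect to the avatar is never executed.
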(event `self.K2_ActivateAbility`
  (bind _character (`/Game/Blueprints/BFL_SoulEater.Get SE Character Base from Actor` (`self.GetAvatarActorFromActorInfo`)))
  (`parent.K2_ActivateAbility`)
  (bind _returnvalue (`self.K2_CommitAbility`))
  (if _returnvalue
    (`/Engine/EditorBlueprintResources/StandardMacros.IsValid` _character
      (:`Is Valid`
        (`Character.Jump` _character))
      (:`Is Not Valid`
        _)))
  (`self.K2_EndAbility`))