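; Water pool hazard that calls OnDead on any actor implementing I_Player that overlaps its Box.
; The construction script tiles an InstancedStaticMesh grid from SizeX, SizeY, Size and Scale, then offsets it toward the actor's center.
; It derives the thin Box trigger's extents from the same dimensions, using full rather than half lengths.
; The kill message goes through the player's SEPlayerMessage, fetched via the interface.
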(event `self.ReceiveActorBeginOverlap`
  (params (OtherActor :type "Actor Object Reference")))

(event `self.Box.OnComponentBeginOverlap`
  (params (OverlappedComponent :type "PrimitiveComponent Object Reference") (OtherActor :type "Actor Object Reference") (OtherComp :type "PrimitiveComponent Object Reference") (OtherBodyIndex :type Integer) (bFromSweep :type Boolean) (SweepResult :type "HitResult Structure (by ref)"))
  (if (`KismetSystemLibrary.DoesImplementInterface` OtherActor "/Game/Blueprints/I_Player.I_Player_C")
    (bind _player (message `/Game/Blueprints/I_Player.Get SE Player` OtherActor))
    (`/Game/Blueprints/BP_CharacterBase.On Dead` _player)))

(fn `UserConstructionScript`
  (set `self.Size Scaled` (* (`self.Size`) (`self.Scale`)))
  (`|ExecutionSequence`
    (:`then_0`
      (for _index (range (+ (`self.Size Y`) 1))
        (for _index_2 (range (+ (`self.Size X`) 1))
          (`InstancedStaticMeshComponent.AddInstance` (`self.InstancedStaticMesh`) (`KismetMathLibrary.MakeTransform` (`KismetMathLibrary.MakeVector` (* _index_2 (`self.Size Scaled`)) (* _index (`self.Size Scaled`))) (struct) (`KismetMathLibrary.Conv_DoubleToVector` (`self.Scale`)))))))
    (:`then_1`
      (`SceneComponent.K2_SetRelativeLocation` (`self.InstancedStaticMesh`) (`KismetMathLibrary.MakeVector` (* (/ (`KismetMathLibrary.Conv_IntToDouble` (`self.Size X`)) -2.0) (`self.Size Scaled`)) (* (/ (`KismetMathLibrary.Conv_IntToDouble` (`self.Size Y`)) -2.0) (`self.Size Scaled`))) false false))
    (:`then_2`
      (`BoxComponent.SetBoxExtent` (`self.Box`) (`KismetMathLibrary.MakeVector` (* (/ (`KismetMathLibrary.Conv_IntToDouble` (`self.Size X`)) 1.0) (`self.Size Scaled`)) (* (/ (`KismetMathLibrary.Conv_IntToDouble` (`self.Size Y`)) 1.0) (`self.Size Scaled`)) 10.0) true))))