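; Base melee Gameplay Ability that plays a montage and applies gameplay effects from its events.
; On activation it commits, then runs PlayMontageAndWaitForEvent listening for Event.Montage tags.
; Each received event passes its tag and data to ApplyEffectContainer; blend out, interruption or cancellation ends the ability, while completion only prints a debug string.
; An older WeaponHit wait that applies GE_PlayerWeaponHit is left unconnected.
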(event `self.K2_ActivateAbility`
  (`parent.K2_ActivateAbility`)
  (bind _returnvalue (`self.K2_CommitAbility`))
  (if _returnvalue
    (bind (_asynctaskproxy _eventtag _eventdata) (`PlayMontageAndWaitForEvent.PlayMontageAndWaitForEvent` "None" (`self.Montage To Play`) (struct :`GameplayTags` (struct :`(TagName` "Event.Montage"))))
      (:`OnCompleted`
        (`KismetSystemLibrary.PrintString` "Melle Ability End"))
      (:`OnBlendOut`
        (`self.K2_EndAbility` :!label _label))
      (:`OnInterrupted`
        (goto _label))
      (:`OnCancelled`
        (goto _label))
      (:`EventReceived`
        (`self.ApplyEffectContainer` _eventtag _eventdata)))))