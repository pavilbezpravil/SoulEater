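; Player gameplay ability for the High Spin move that closes the gap to the player's current target.
; On activation it runs the parent logic, then gets the player and its TargetActor through GetSEPlayerMessage on the avatar.
; If both are valid, MoveToLocation carries the player over a short fixed duration to a point offset just short of the target along the line between them.
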(event `self.K2_ActivateAbility`
  (`parent.K2_ActivateAbility`)
  (bind _player (message `/Game/Blueprints/I_Player.Get SE Player` (`self.GetAvatarActorFromActorInfo`)))
  (`/Engine/EditorBlueprintResources/StandardMacros.IsValid` _player
    (:`Is Valid`
      (bind _target_actor (`/Game/Blueprints/BP_Player.Target Actor` _player))
      (`/Engine/EditorBlueprintResources/StandardMacros.IsValid` _target_actor
        (:`Is Valid`
          (bind _returnvalue (`Actor.K2_GetActorLocation` _target_actor))
          (`AbilityTask_MoveToLocation.MoveToLocation` "None" (+ _returnvalue (* (`KismetMathLibrary.Normal` (- _returnvalue (`Actor.K2_GetActorLocation` _player))) -200.0)) 0.3))))))