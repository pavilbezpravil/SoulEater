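; Base weapon actor that acts as a melee hitbox and reports hits to its wielder through Gameplay Ability System events.
; BeginWeaponAttack stores the supplied attack tag and enables capsule collision, and EndWeaponAttack disables it.
; Capsule overlaps with any actor other than the instigator send a gameplay event with that tag to the instigator, carrying the hit actor as target.
; The weapon applies no damage itself.
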(event `self.ReceiveBeginPlay`
  (`PrimitiveComponent.IgnoreActorWhenMoving` (`self.Capsule`) null true)
  (`PrimitiveComponent.IgnoreActorWhenMoving` (`self.Capsule`) (`self.GetInstigator`) true))

(event `Event Begin Weapon Attack`
  (params (Tag :type "GameplayTag Structure"))
  (set `self.Atatck Tag` Tag)
  (set `self.Is Attacking` true)
  (`PrimitiveComponent.SetCollisionEnabled` (`self.Capsule`) "QueryAndPhysics"))

(event `Event End Weapon Attack`
  (set `self.Is Attacking` false)
  (`PrimitiveComponent.SetCollisionEnabled` (`self.Capsule`) "NoCollision"))

(event `self.Capsule.OnComponentBeginOverlap`
  (params (OverlappedComponent :type "PrimitiveComponent Object Reference") (OtherActor :type "Actor Object Reference") (OtherComp :type "PrimitiveComponent Object Reference") (OtherBodyIndex :type Integer) (bFromSweep :type Boolean) (SweepResult :type "HitResult Structure (by ref)"))
  (if (!= OtherActor (`self.GetInstigator`))
    (`AbilitySystemBlueprintLibrary.SendGameplayEventToActor` (`self.GetInstigator`) (`self.Atatck Tag`) (make `GameplayEventData` (struct) (`self.GetInstigator`) OtherActor))))

(fn `UserConstructionScript`)