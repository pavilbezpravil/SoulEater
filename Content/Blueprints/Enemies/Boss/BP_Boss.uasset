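; BP_Boss is a boss enemy character that fights with a sword and uses the Gameplay Ability System.
; On BeginPlay it sets up the sword weapon and assigns its right capsule as the weapon's collision primitive.
; Melee attacks activate the GA_BOSS_HIT1 ability, while damage handling defers to the parent class.
; Helper functions report the attacking tag and whether stamina is below a fixed threshold.
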(event `self.ReceiveBeginPlay`
  (`parent.ReceiveBeginPlay`)
  (set `self.Weapon Class` "/Game/Blueprints/Enemies/Boss/BP_BossSword.BP_BossSword_C")
  (`self.Set Weapon` "sword")
  (`/Game/Blueprints/BP_WeaponBase.Set Collisoin Primitive` (`self.CurrentWeapon`) (`self.Right Capsule`)))

(event `self.OnDamaged`
  (params (DamageAmount :type "Float (single-precision)") (HitInfo :type "HitResult Structure (by ref)") (DamageTags :type "GameplayTagContainer Structure (by ref)") (InstigatorCharacter :type "SECharacterBase Object Reference") (DamageCauser :type "Actor Object Reference"))
  (`parent.OnDamaged` DamageAmount HitInfo DamageTags InstigatorCharacter DamageCauser))

(event `/Game/Blueprints/I_Melle.MelleAttack`
  (params (DistanceToPlayer :type "Float (single-precision)"))
  (`AbilitySystemComponent.TryActivateAbilityByClass` (`self.AbilitySystemComponent`) "/Game/Abilities/Enemies/BOSS/GA_BOSS_HIT1.GA_BOSS_HIT1_C" true))

(fn `InAttack`
  (returns (InAttack :type Boolean))
  (return (`self.HasTag` (struct :`TagName` "Abilities.Attacking"))))

(fn `InStamina`
  (returns (InStamina :type Boolean))
  (return (< (`self.GetStamina`) 75.0)))

(fn `UserConstructionScript`
  (`parent.UserConstructionScript`))