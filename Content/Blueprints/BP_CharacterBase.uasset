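; Base character Blueprint that handles weapon attachment to mesh sockets and montage-driven melee-style combo attacks.
; Combo input calls the empty StartCombo stub, or, with the Abilities.Attacking tag, continues only during an open input window.
; Continuing links the active montage section to NextComboAttackNS's next section and jumps to the current section's end, ending the combo when none is named.
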(event `self.ReceiveBeginPlay`)

(event `Equip Weapon`
  (params (Weapon :type "/Game/Blueprints/BP_WeaponBase Object Reference") (SocketName :type Name))
  (bind _output_get (set `self.CurrentWeapon` Weapon))
  (`self.K2_AttachToComponent` _output_get (`self.Mesh`) SocketName "SnapToTarget" "SnapToTarget" "KeepRelative" true))

(event `Event Combo End`
  (set `self.Is Wait Continue Combo Requirements` false)
  (set `self.Receive Combo Requarements` false))

(event `Begin Wait Continue Combo Requirement`
  (set `self.Is Wait Continue Combo Requirements` true))

(event `End Wait Continue Combo Requirement`
  (set `self.Is Wait Continue Combo Requirements` false))

(event `Recieve Combo Input`
  (if (`self.HasTag` (struct :`TagName` "Abilities.Attacking"))
    (if (`self.Is Wait Continue Combo Requirements`)
      (set `self.Receive Combo Requarements` true)
      (`self.Continue Combo`))
    (else
      (`self.Start Combo`))))

(event `Continue Combo`
  (bind _returnvalue (`SkeletalMeshComponent.GetAnimInstance` (`self.Mesh`)))
  (bind _returnvalue_2 (`AnimInstance.GetCurrentActiveMontage` _returnvalue))
  (bind _returnvalue_3 (`AnimInstance.Montage_GetCurrentSection` _returnvalue _returnvalue_2))
  (if (!= (`/Game/Blueprints/AnimNotifies/NextComboAttackNS.Next Section` (`self.Next Combo Attack NS`)) "None")
    (`AnimInstance.Montage_SetNextSection` _returnvalue _returnvalue_3 (`/Game/Blueprints/AnimNotifies/NextComboAttackNS.Next Section` (`self.Next Combo Attack NS`)) _returnvalue_2)
    (`AnimInstance.Montage_JumpToSectionsEnd` _returnvalue _returnvalue_3 _returnvalue_2)
    (else
      (`self.Event Combo End`))))

(event `Start Combo`)

(fn `UserConstructionScript`)