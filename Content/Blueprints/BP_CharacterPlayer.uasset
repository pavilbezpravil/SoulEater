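; Player character Blueprint that connects Gameplay Ability System actions and attribute changes to the player controller.
; The Jump input and a second input event activate the GA_Jump and GA_Heal abilities through the AbilitySystemComponent.
; Health, stamina and souls change events call their parent handlers, then notify the SE player controller to refresh, as BeginPlay does for all three.
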(event `self.ReceiveBeginPlay`
  (`self.Update Controller Souls`)
  (`self.Update Controller Health`)
  (`self.Update Controller Stamina`))

(event `InputAction|Jump`
  (params (Key :type "Key Structure"))
  (:`Pressed`
    (bind _returnvalue (`AbilitySystemComponent.TryActivateAbilityByClass` (`self.AbilitySystemComponent`) "/Game/Abilities/GA_Jump.GA_Jump_C" true))
    (if _returnvalue
      (`KismetSystemLibrary.PrintString` "Jump"))))

(event `Receive Input`
  (`AbilitySystemComponent.TryActivateAbilityByClass` (`self.AbilitySystemComponent`) "/Game/Abilities/GA_Heal.GA_Heal_C" true))

(event `self.OnHealthChanged`
  (params (DeltaValue :type "Float (single-precision)") (EventTags :type "GameplayTagContainer Structure (by ref)"))
  (`parent.OnHealthChanged` DeltaValue EventTags)
  (`self.Update Controller Health`))

(event `self.OnStaminaChanged`
  (params (DeltaValue :type "Float (single-precision)") (EventTags :type "GameplayTagContainer Structure (by ref)"))
  (`parent.OnStaminaChanged` DeltaValue EventTags)
  (`self.Update Controller Stamina`))

(event `self.OnSoulsChanged`
  (params (DeltaValue :type "Float (single-precision)") (EventTags :type "GameplayTagContainer Structure (by ref)"))
  (`parent.OnSoulsChanged` DeltaValue EventTags)
  (`self.Update Controller Souls`))

(fn `Update Controller Health`
  (`/Game/Blueprints/BP_PlayerController.On Health Changed` (`/Game/Blueprints/BFL_SoulEater.Get SE Player Controller` self)))

(fn `Update Controller Souls`
  (`/Game/Blueprints/BP_PlayerController.On Souls Changed` (`/Game/Blueprints/BFL_SoulEater.Get SE Player Controller` self)))

(fn `Update Controller Stamina`
  (`/Game/Blueprints/BP_PlayerController.Update Stamina Bar` (`/Game/Blueprints/BFL_SoulEater.Get SE Player Controller` self)))

(fn `UserConstructionScript`)