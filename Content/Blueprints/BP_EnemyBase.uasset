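; BP_EnemyBase is a base enemy Blueprint that handles target feedback and weapon equipping.
; When targeted, it attaches a Niagara effect bound to its skeletal mesh and shows the HP widget.
; Losing the target deactivates and clears that effect and, only if the effect was valid, hides the widget.
; SetWeapon spawns the configured weapon class with itself as instigator and equips it to a given socket.
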(event `self.ReceiveBeginPlay`)

(event `/Game/Blueprints/I_Target.OnTarget`
  (bind _returnvalue (`NiagaraFunctionLibrary.SpawnSystemAttached` "/Game/FX/Target/NS_Target.NS_Target" (`self.Mesh`) "None" (0.0 0.0 0.0) (struct) "KeepRelativeOffset"))
  (bind _output_get (set `self.Target FX` _returnvalue))
  (`NiagaraFunctionLibrary.OverrideSystemUserVariableSkeletalMeshComponent` _output_get "Skeletal Mesh" (`self.Mesh`))
  (`self.Show HP Widget`))

(event `/Game/Blueprints/I_Target.OnLoseTarget`
  (`/Engine/EditorBlueprintResources/StandardMacros.IsValid` (`self.Target FX`)
    (:`Is Valid`
      (`ActorComponent.Deactivate` (`self.Target FX`))
      (set `self.Target FX` null)
      (`self.Hide HP Widget`))))

(fn `Set Weapon`
  (params (SocketName :type Name))
  (if (`KismetSystemLibrary.IsValidClass` (`self.Weapon Class`))
    (bind _returnvalue (`|SpawnActorFromClass` (`self.Weapon Class`) (`KismetMathLibrary.MakeTransform` (0.0 0.0 0.0)) "Undefined" "OverrideRootScale" null self))
    (`self.Equip Weapon` _returnvalue SocketName)))

(fn `UserConstructionScript`
  (`parent.UserConstructionScript`))