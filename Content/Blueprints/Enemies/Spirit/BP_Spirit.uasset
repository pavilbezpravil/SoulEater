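; BP_Spirit is a Spirit enemy character that drives its combat actions through the Gameplay Ability System.
; On BeginPlay it sets a weapon on the right-side socket and assigns the right capsule as that weapon's collision primitive.
; Taking damage runs the parent handling, then triggers the impact ability if the Spirit is still valid.
; Melee attacks choose between a close-range hit ability and a standard hit ability based on distance to the player.
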(event `self.ReceiveBeginPlay`
  (`self.Set Weapon` "s_r_socket")
  (`/Game/Blueprints/BP_WeaponBase.Set Collisoin Primitive` (`self.CurrentWeapon`) (`self.Right Capsule`)))

(event `self.OnDamaged`
  (params (DamageAmount :type "Float (single-precision)") (HitInfo :type "HitResult Structure (by ref)") (DamageTags :type "GameplayTagContainer Structure (by ref)") (InstigatorCharacter :type "SECharacterBase Object Reference") (DamageCauser :type "Actor Object Reference"))
  (`parent.OnDamaged` DamageAmount HitInfo DamageTags InstigatorCharacter DamageCauser)
  (`/Engine/EditorBlueprintResources/StandardMacros.IsValid` self
    (:`Is Valid`
      (`AbilitySystemComponent.TryActivateAbilityByClass` (`self.AbilitySystemComponent`) "/Game/Abilities/Enemies/Spirit/GA_SpiritImpact.GA_SpiritImpact_C" true))))

(event `/Game/Blueprints/I_Melle.MelleAttack`
  (params (DistanceToPlayer :type "Float (single-precision)"))
  (bind _abilitysystemcomponent (`self.AbilitySystemComponent`))
  (if (< DistanceToPlayer 150.0)
    (`AbilitySystemComponent.TryActivateAbilityByClass` _abilitysystemcomponent "/Game/Abilities/Enemies/Spirit/GA_SpiritHit_Close.GA_SpiritHit_Close_C" true)
    (else
      (`AbilitySystemComponent.TryActivateAbilityByClass` _abilitysystemcomponent "/Game/Abilities/Enemies/Spirit/GA_SpiritHit.GA_SpiritHit_C" true))))

(fn `UserConstructionScript`
  (`parent.UserConstructionScript`))