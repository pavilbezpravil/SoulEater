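; Anim notify state that marks the window in an attack animation for continuing a combo on BP_CharacterBase owners.
; On begin, it calls BeginWaitContinueComboRequirement on the character and stores itself in the character's NextComboAttackNS variable.
; On end, it calls EndWaitContinueComboRequirement and clears that reference.
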(fn `Received_NotifyBegin`
  (params (MeshComp :type "SkeletalMeshComponent Object Reference") (Animation :type "AnimSequenceBase Object Reference") (TotalDuration :type "Float (double-precision)"))
  (returns (ReturnValue :type Boolean))
  (bind _asbp_character_base (cast `/Game/Blueprints/BP_CharacterBase` (`ActorComponent.GetOwner` MeshComp)))
  (`/Game/Blueprints/BP_CharacterBase.Begin Wait Continue Combo Requirement` _asbp_character_base)
  (set `/Game/Blueprints/BP_CharacterBase.Next Combo Attack NS` self _asbp_character_base)
  (return true))

(fn `Received_NotifyEnd`
  (params (MeshComp :type "SkeletalMeshComponent Object Reference") (Animation :type "AnimSequenceBase Object Reference"))
  (returns (ReturnValue :type Boolean))
  (bind _asbp_character_base (cast `/Game/Blueprints/BP_CharacterBase` (`ActorComponent.GetOwner` MeshComp)))
  (`/Game/Blueprints/BP_CharacterBase.End Wait Continue Combo Requirement` _asbp_character_base)
  (set `/Game/Blueprints/BP_CharacterBase.Next Combo Attack NS` null _asbp_character_base)
  (return true))