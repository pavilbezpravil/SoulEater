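; Player controller that owns the player HUD (health, stamina and souls widgets) and forwards attack input to the possessed BP_Player.
; On possess it creates the widgets once, caches the character and shows them; on unpossess it clears the reference and hides them.
; Change events for health, stamina and souls read the character's values and push bar ratios or a truncated souls count to the widgets.
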(event `self.ReceivePossess`
  (params (PossessedPawn :type "Pawn Object Reference"))
  (`self.Create WBP`)
  (bind _asbp_player (cast `/Game/Blueprints/BP_Player` PossessedPawn))
  (set `self.Controlled Character` _asbp_player)
  (`self.Show WBP`))

(event `self.ReceiveUnPossess`
  (params (UnpossessedPawn :type "Pawn Object Reference"))
  (set `self.Controlled Character` null)
  (`self.Hide WBP`))

(event `On Health Changed`
  (`self.Update Health Bar`))

(event `On Stamina Changed`
  (`self.Update Stamina Bar`))

(event `On Souls Changed`
  (`self.Update Souls`))

(event `InputAction|Attack`
  (params (Key :type "Key Structure"))
  (:`Pressed`
    (`self.Valid Controlled Character`
      (:`Valid`
        (`/Game/Blueprints/BP_Player.Receive Input` (`self.Controlled Character`))))))

(fn `Create WBP`
  (if (not (`self.Is WBP Created`))
    (`|ExecutionSequence`
      (:`then_0`
        (bind _returnvalue (`|CreateWidget` "/Game/Blueprints/WidgetsBP/WBP_HealthBar.WBP_HealthBar_C" self))
        (bind _output_get (set `self.Health Bar` _returnvalue))
        (`UserWidget.AddToViewport` _output_get 0))
      (:`then_1`
        (bind _returnvalue_2 (`|CreateWidget` "/Game/Blueprints/WidgetsBP/WBP_Souls.WBP_Souls_C" self))
        (bind _output_get_2 (set `self.Souls` _returnvalue_2))
        (`UserWidget.AddToViewport` _output_get_2 0))
      (:`then_2`
        (bind _returnvalue_3 (`|CreateWidget` "/Game/Blueprints/WidgetsBP/WBP_StaminaBar.WBP_StaminaBar_C" self))
        (bind _output_get_3 (set `self.Stamin Bar` _returnvalue_3))
        (`UserWidget.AddToViewport` _output_get_3 0))
      (:`then_3`
        (set `self.Is WBP Created` true)))))

(fn `Hide WBP`
  (`Widget.SetVisibility` (`self.Health Bar`) "Hidden")
  (`Widget.SetVisibility` (`self.Souls`) "Hidden")
  (`Widget.SetVisibility` (`self.Stamin Bar`) "Hidden"))

(fn `Show WBP`
  (`Widget.SetVisibility` (`self.Health Bar`) "Visible")
  (`Widget.SetVisibility` (`self.Souls`) "Visible")
  (`Widget.SetVisibility` (`self.Stamin Bar`) "Visible"))

(fn `Update Health Bar`
  (bind _controlled_character (`self.Controlled Character`))
  (`/Game/Blueprints/WidgetsBP/WBP_HealthBar.Update Bar` (`self.Health Bar`) (/ (`SECharacterBase.GetHealth` _controlled_character) (`SECharacterBase.GetMaxHealth` _controlled_character))))

(fn `Update Souls`
  (`/Game/Blueprints/WidgetsBP/WBP_Souls.Update Souls` (`self.Souls`) (`KismetMathLibrary.FTrunc` (`SECharacterBase.GetSouls` (`self.Controlled Character`)))))

(fn `Update Stamina Bar`
  (bind _controlled_character (`self.Controlled Character`))
  (`/Game/Blueprints/WidgetsBP/WBP_StaminaBar.Update Bar` (`self.Stamin Bar`) (/ (`SECharacterBase.GetStamina` _controlled_character) (`SECharacterBase.GetMaxStamina` _controlled_character))))

(fn `UserConstructionScript`)