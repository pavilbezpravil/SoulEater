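; Player character for a souls-style action game built on the Gameplay Ability System, with combos, jump or dodge, and lock-on targeting.
; Holding ChooseTarget applies a targeting effect, sphere-traces for I_Target actors and turns the camera toward the target; Whip lerps the player there.
; Tick converts movement into forward/backward tag effects that pick the combo ability.
; Health, stamina and soul changes are forwarded to the controller, and a starting weapon is equipped at BeginPlay.
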(event `self.ReceiveTick`
  (params (DeltaSeconds :type "Float (single-precision)"))
  (`|ExecutionSequence`
    (:`then_0`
      (if (`self.IsTargeting`)
        (`/Engine/EditorBlueprintResources/StandardMacros.IsValid` (`self.Target Actor`)
          (:`Is Not Valid`
            (bind _actors (`self.Look For Target`))
            (`self.Choose Target From Actors` _actors)))))
    (:`then_1`
      (`self.Apply Input Tags`))
    (:`then_2`
      (`self.Camera To Target`))))

(event `self.ReceiveBeginPlay`
  (bind _weapon_classes (`self.Weapon Classes`))
  (`parent.ReceiveBeginPlay`)
  (`|ExecutionSequence`
    (:`then_0`
      (if (`KismetMathLibrary.Conv_IntToBool` (`KismetArrayLibrary.Array_Length` _weapon_classes))
        (bind _returnvalue (`|SpawnActorFromClass` (`|GetArrayItem` _weapon_classes) (`KismetMathLibrary.MakeTransform` (0.0 0.0 0.0)) "Undefined" "OverrideRootScale" null self))
        (`self.Equip Weapon` _returnvalue "RightHandSocket")))
    (:`then_1`
      (`self.Update Controller Souls`)
      (`self.Update Controller Health`)
      (`self.Update Controller Stamina`))))

(event `InputAction|Jump`
  (params (Key :type "Key Structure"))
  (:`Pressed`
    (if (`self.IsTargeting`)
      (`self.Dodge`)
      (else
        (`AbilitySystemComponent.TryActivateAbilityByClass` (`self.AbilitySystemComponent`) "/Game/Abilities/GA_Jump.GA_Jump_C" true)))))

(event `self.OnLanded`
  (params (Hit :type "HitResult Structure (by ref)"))
  (`AbilitySystemComponent.RemoveActiveEffectsWithGrantedTags` (`self.AbilitySystemComponent`) (struct :`GameplayTags` (struct :`(TagName` "Status.Jumping")))))

(event `InputAction|Whip`
  (params (Key :type "Key Structure"))
  (:`Pressed`
    (`self.Move To Soul`)))

(event `self.OnHealthChanged`
  (params (DeltaValue :type "Float (single-precision)") (EventTags :type "GameplayTagContainer Structure (by ref)"))
  (`parent.OnHealthChanged` DeltaValue EventTags)
  (`self.Update Controller Health`))

(event `self.OnStaminaChanged`
  (params (DeltaValue :type "Float (single-precision)") (EventTags :type "GameplayTagContainer Structure (by ref)"))
  (`parent.OnStaminaChanged` DeltaValue EventTags)
  (`self.Update Controller Stamina`))

(event `self.OnSoulsChanged`
  (params (DeltaValue :type "Float (single-precision)") (EventTags :type "GameplayTagContainer Structure (by ref)"))
  (`parent.OnSoulsChanged` DeltaValue EventTags)
  (`self.Update Controller Souls`))

(event `self.OnDamaged`
  (params (DamageAmount :type "Float (single-precision)") (HitInfo :type "HitResult Structure (by ref)") (DamageTags :type "GameplayTagContainer Structure (by ref)") (InstigatorCharacter :type "SECharacterBase Object Reference") (DamageCauser :type "Actor Object Reference"))
  (`parent.OnDamaged` DamageAmount HitInfo DamageTags InstigatorCharacter DamageCauser)
  (`/Engine/EditorBlueprintResources/StandardMacros.IsValid` self
    (:`Is Valid`
      (`AbilitySystemComponent.TryActivateAbilityByClass` (`self.AbilitySystemComponent`) "/Game/Abilities/Player/GA_PlayerImpact.GA_PlayerImpact_C" true))))

(event `self.On Dead`
  (`parent.On Dead`))

(event `InputAction|ChooseTarget`
  (params (Key :type "Key Structure"))
  (bind _target_actor (`self.Target Actor`))
  (:`Pressed`
    (bind _returnvalue (`AbilitySystemComponent.BP_ApplyGameplayEffectToTarget` :`self` (`self.AbilitySystemComponent`) :`GameplayEffectClass` "/Game/Abilities/Player/GE_Targeting.GE_Targeting_C" :`Target` (`self.AbilitySystemComponent`)))
    (set `self.Targeting Handler` _returnvalue)
    (bind _actors (`self.Look For Target`))
    (`self.Choose Target From Actors` _actors)
    (set `self.bUseControllerRotationYaw` true))
  (:`Released`
    (`AbilitySystemComponent.RemoveActiveGameplayEffect` (`self.AbilitySystemComponent`) (`self.Targeting Handler`) -1)
    (`|ExecutionSequence`
      (:`then_0`
        (`/Engine/EditorBlueprintResources/StandardMacros.IsValid` _target_actor
          (:`Is Valid`
            (message `/Game/Blueprints/I_Target.OnLoseTarget` _target_actor)
            (set `self.bUseControllerRotationYaw` false))))
      (:`then_1`
        (set `self.Target Actor` null)))))

(event `Receive Input`
  (`self.Recieve Combo Input`))

(event `self.Start Combo`
  (if (`self.HasTag` (struct :`TagName` "Input.Forward"))
    (`AbilitySystemComponent.TryActivateAbilityByClass` (`self.AbilitySystemComponent`) "/Game/Abilities/Player/GA_HighSpin.GA_HighSpin_C" true)
    (elif (`self.HasTag` (struct :`TagName` "Input.Backward"))
      (`AbilitySystemComponent.TryActivateAbilityByClass` (`self.AbilitySystemComponent`) "/Game/Abilities/Player/GA_ToAir.GA_ToAir_C" true)
      (else
        (`AbilitySystemComponent.TryActivateAbilityByClass` (`self.AbilitySystemComponent`) "/Game/Abilities/Player/GA_SimpleCombo.GA_SimpleCombo_C" true)))))

(event `Dodge`
  (`AbilitySystemComponent.TryActivateAbilityByClass` (`self.AbilitySystemComponent`) "/Game/Abilities/Player/GA_Dodge.GA_Dodge_C" true))

(event `Catch Souls`
  (params (NewParam :type Integer))
  (bind _output_get (set `self.Souls` (+ (`self.Souls`) NewParam)))
  (`KismetSystemLibrary.PrintString` (`KismetStringLibrary.Conv_IntToString` _output_get)))

(event `Move To Soul`
  (bind _target_actor (`self.Target Actor`))
  (`/Engine/EditorBlueprintResources/StandardMacros.IsValid` _target_actor
    (:`Is Valid`
      (set `self.Move To Soul Target Loc` (`self.K2_GetActorLocation` _target_actor))
      (set `self.Move To Soul Start Loc` (`self.K2_GetActorLocation`))
      (`TimelineComponent.SetPlayRate` (`self.Timeline_0`) 1.0)
      (bind (_direction _newtrack_0) (`Timeline|Timeline_0` :!via `PlayFromStart`)
        (:`Update`
          (`self.K2_SetActorLocation` (`KismetMathLibrary.VLerp` (`self.Move To Soul Start Loc`) (`self.Move To Soul Target Loc`) _newtrack_0)))
        (:`Finished`
          (`self.Disable Movement` true 1.0))))))

(fn `Apply Input Tags`
  (bind _returnvalue (`self.GetVelocity`))
  (bind _abilitysystemcomponent (`self.AbilitySystemComponent`))
  (bind _abilitysystemcomponent_2 (`self.AbilitySystemComponent`))
  (if (and (> (`KismetMathLibrary.VSize` (`self.GetLastMovementInputVector`)) 0.25) (> (`KismetMathLibrary.VSize` _returnvalue) 0.25))
    (if (> (`KismetMathLibrary.Dot_VectorVector` _returnvalue (`self.GetActorForwardVector`)) 100.0)
      (`AbilitySystemComponent.BP_ApplyGameplayEffectToTarget` :`self` _abilitysystemcomponent_2 :`GameplayEffectClass` "/Game/Abilities/Player/Combo/GE_Input_Forward.GE_Input_Forward_C" :`Target` _abilitysystemcomponent_2)
      (else
        (`AbilitySystemComponent.BP_ApplyGameplayEffectToTarget` :`self` _abilitysystemcomponent :`GameplayEffectClass` "/Game/Abilities/Player/Combo/GE_Input_Backward.GE_Input_Backward_C" :`Target` _abilitysystemcomponent)))))

(fn `Camera To Target`
  (bind _returnvalue (`Controller.GetControlRotation` (`self.GetController`)))
  (`/Engine/EditorBlueprintResources/StandardMacros.IsValid` (`self.Target Actor`)
    (:`Is Valid`
      (`Controller.SetControlRotation` (`self.GetController`) (`KismetMathLibrary.MakeRotator` (.roll _returnvalue) (.pitch (`KismetMathLibrary.RInterpTo` _returnvalue (`KismetMathLibrary.FindLookAtRotation` (`self.K2_GetActorLocation`) (`self.K2_GetActorLocation` (`self.Target Actor`))) (`GameplayStatics.GetWorldDeltaSeconds`) 3.0)) (.yaw (`KismetMathLibrary.RInterpTo` _returnvalue (`KismetMathLibrary.FindLookAtRotation` (`self.K2_GetActorLocation`) (`self.K2_GetActorLocation` (`self.Target Actor`))) (`GameplayStatics.GetWorldDeltaSeconds`) 3.0)))))))

(fn `Choose Target From Actors`
  (params (NewParam :type "Array of Actor Object Reference"))
  (if (> (`KismetArrayLibrary.Array_Length` NewParam) 0)
    (bind _output_get (set `self.Target Actor` (`|GetArrayItem` NewParam)))
    (message `/Game/Blueprints/I_Target.OnTarget` _output_get)))

(fn `Get SE Player`
  (returns (Player :type "/Game/Blueprints/BP_Player Object Reference"))
  (return self))

(fn `IsTargeting`
  (returns (NewParam :type Boolean))
  (return (`self.HasTag` (struct :`TagName` "Status.Targeting"))))

(fn `Look For Target`
  (returns (Actors :type "Array of Actor Object Reference"))
  (locals (NewLocalVar_0 :type Boolean) (TmpActors :type "Array of Actor Object Reference"))
  (bind _returnvalue (`self.K2_GetActorLocation`))
  (bind _outhits (`KismetSystemLibrary.SphereTraceMultiForObjects` _returnvalue (+ _returnvalue (* (`KismetMathLibrary.GetForwardVector` (`KismetMathLibrary.MakeRotator` (.roll (`Controller.GetControlRotation` (`self.GetController`))) (.pitch (`Controller.GetControlRotation` (`self.GetController`))) (.yaw (`Controller.GetControlRotation` (`self.GetController`))))) 1500.0)) 300.0 (`|MakeArray` "ObjectTypeQuery3" "ObjectTypeQuery1" "ObjectTypeQuery2" :!type "EObjectTypeQuery Enum")))
  (for _array_element _outhits
    (if (`KismetSystemLibrary.DoesImplementInterface` (`.HitActor` (`GameplayStatics.BreakHitResult` _array_element)) "/Game/Blueprints/I_Target.I_Target_C")
      (`KismetArrayLibrary.Array_AddUnique` (`local.TmpActors`) (`.HitActor` (`GameplayStatics.BreakHitResult` _array_element)))))
  (return (`local.TmpActors`)))

(fn `Move To Target`
  (`/Engine/EditorBlueprintResources/StandardMacros.IsValid` (`self.Target Actor`)
    (:`Is Valid`
      (`self.LaunchCharacter` (0.0 0.0 0.0)))))

(fn `Update Controller Health`
  (bind _asbp_player_controller (`/Game/Blueprints/BFL_SoulEater.Get SE Pawn Controller` self))
  (`/Engine/EditorBlueprintResources/StandardMacros.IsValid` _asbp_player_controller
    (:`Is Valid`
      (`/Game/Blueprints/BP_PlayerController.On Health Changed` _asbp_player_controller))))

(fn `Update Controller Souls`
  (bind _asbp_player_controller (`/Game/Blueprints/BFL_SoulEater.Get SE Pawn Controller` self))
  (`/Engine/EditorBlueprintResources/StandardMacros.IsValid` _asbp_player_controller
    (:`Is Valid`
      (`/Game/Blueprints/BP_PlayerController.On Souls Changed` _asbp_player_controller))))

(fn `Update Controller Stamina`
  (bind _asbp_player_controller (`/Game/Blueprints/BFL_SoulEater.Get SE Pawn Controller` self))
  (`/Engine/EditorBlueprintResources/StandardMacros.IsValid` _asbp_player_controller
    (:`Is Valid`
      (`/Game/Blueprints/BP_PlayerController.Update Stamina Bar` _asbp_player_controller))))

(fn `UserConstructionScript`)