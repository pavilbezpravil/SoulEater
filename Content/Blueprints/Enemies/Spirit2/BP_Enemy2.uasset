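; BP_Enemy2 is a spear-wielding Spirit2 enemy that uses the Gameplay Ability System for its combat actions.
; It equips the spear on BeginPlay, activates a hit ability for melee attacks and triggers an impact ability when damaged.
; Helper functions report whether it carries the attacking tag and whether stamina is below a fixed threshold.
; Tick prints current stamina as debug output.
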(event `self.ReceiveBeginPlay`
  (`parent.ReceiveBeginPlay`)
  (set `self.Weapon Class` "/Game/Blueprints/Enemies/Spirit2/BP_SPEAR.BP_SPEAR_C")
  (`self.Set Weapon` "Spear"))

(event `self.OnDamaged`
  (params (DamageAmount :type "Float (single-precision)") (HitInfo :type "HitResult Structure (by ref)") (DamageTags :type "GameplayTagContainer Structure (by ref)") (InstigatorCharacter :type "SECharacterBase Object Reference") (DamageCauser :type "Actor Object Reference"))
  (`parent.OnDamaged` DamageAmount HitInfo DamageTags InstigatorCharacter DamageCauser)
  (`/Engine/EditorBlueprintResources/StandardMacros.IsValid` self
    (:`Is Valid`
      (`AbilitySystemComponent.TryActivateAbilityByClass` (`self.AbilitySystemComponent`) "/Game/Abilities/Enemies/Spirit2/GA_Spirit2Impact.GA_Spirit2Impact_C" true))))

(event `/Game/Blueprints/I_Melle.MelleAttack`
  (params (DistanceToPlayer :type "Float (single-precision)"))
  (`AbilitySystemComponent.TryActivateAbilityByClass` (`self.AbilitySystemComponent`) "/Game/Abilities/Enemies/Spirit2/GA_Spirit2Hit.GA_Spirit2Hit_C" true))

(event `self.ReceiveTick`
  (params (DeltaSeconds :type "Float (single-precision)"))
  (`KismetSystemLibrary.PrintString` (`KismetStringLibrary.Conv_DoubleToString` (`self.GetStamina`))))

(fn `InAttack`
  (returns (InAttack :type Boolean))
  (return (`self.HasTag` (struct :`TagName` "Abilities.Attacking"))))

(fn `InStamina`
  (returns (InStamina :type Boolean))
  (return (< (`self.GetStamina`) 75.0)))

(fn `UserConstructionScript`)