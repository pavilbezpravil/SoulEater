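; SEGameInstance is the game instance that owns the SESave object and handles loading, saving and deleting it in a single slot.
; On Init it sets DevelopMode whenever the current level is not L_StartLevel, then loads the existing save or creates a fresh one.
; DevelopMode skips the disk load and, after a short delay, calls StartGame on the player controller.
; Deleting the slot also replaces the in-memory save with a new object.
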(event `Delete Save`
  (`GameplayStatics.DeleteGameInSlot` (`self.Game Save Slot Name`))
  (set `self.Has Game Save` false)
  (bind _returnvalue (`GameplayStatics.CreateSaveGameObject` "/Game/Blueprints/Save/SESave.SESave_C"))
  (set `self.Game Save` _returnvalue))

(event `Save Game`
  (bind _returnvalue (`GameplayStatics.SaveGameToSlot` (`self.Game Save`) (`self.Game Save Slot Name`)))
  (if (not _returnvalue)
    (`KismetSystemLibrary.PrintString` "Cant save game")))

(event `Load Save`
  (if (not (`self.Develop Mode`))
    (bind _returnvalue (`GameplayStatics.DoesSaveGameExist` (`self.Game Save Slot Name`)))
    (bind _output_get (set `self.Has Game Save` _returnvalue))
    (if _output_get
      (bind _returnvalue_2 (`GameplayStatics.LoadGameFromSlot` (`self.Game Save Slot Name`)))
      (bind _assesave (cast `/Game/Blueprints/Save/SESave` _returnvalue_2)
        (:`then`
          (set `self.Game Save` _assesave))
        (:`CastFailed`
          (`KismetSystemLibrary.PrintString` "Canr cast to SEGameSave")))
      (else
        (bind _returnvalue_3 (`GameplayStatics.CreateSaveGameObject` "/Game/Blueprints/Save/SESave.SESave_C" :!label _label))
        (set `self.Game Save` _returnvalue_3)
        (if (`self.Develop Mode`)
          (`KismetSystemLibrary.Delay` 0.2)
          (`/Game/Blueprints/BP_PlayerController.Start Game` (`/Game/Blueprints/BFL_SoulEater.Get SE Player Controller` self)))))
    (else
      (set `self.Has Game Save` false)
      (goto _label))))

(event `self.ReceiveInit`
  (bind _returnvalue (`GameplayStatics.GetCurrentLevelName` true))
  (set `self.Develop Mode` (`KismetStringLibrary.NotEqual_StrStr` _returnvalue "L_StartLevel"))
  (`self.Load Save`))