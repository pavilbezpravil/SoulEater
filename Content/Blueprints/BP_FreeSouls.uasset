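; BP_FreeSouls is a souls pickup that grants its Souls to an overlapping actor implementing I_Player.
; On sphere overlap it attaches a souls Niagara effect to that actor, passing in its own location, then calls CatchSouls, spawns a death effect and destroys itself.
; OnTarget spawns a fire emitter at the pickup, which is removed when the target is lost or the actor is destroyed.
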(event `self.ReceiveBeginPlay`
  (add `self.OnDestroyed` (delegate `OnDestroyed_Event_0`)))

(event `OnDestroyed_Event_0` :!signature `self.OnDestroyed`
  (params (DestroyedActor :type "Actor Object Reference"))
  (`self.Delete Target FX`))

(event `self.Sphere.OnComponentBeginOverlap`
  (params (OverlappedComponent :type "PrimitiveComponent Object Reference") (OtherActor :type "Actor Object Reference") (OtherComp :type "PrimitiveComponent Object Reference") (OtherBodyIndex :type Integer) (bFromSweep :type Boolean) (SweepResult :type "HitResult Structure (by ref)"))
  (`/Engine/EditorBlueprintResources/StandardMacros.IsValid` OtherActor
    (:`Is Valid`
      (if (`KismetSystemLibrary.DoesImplementInterface` OtherActor "/Game/Blueprints/I_Player.I_Player_C")
        (`self.Spawn Souls FX Attached` OtherActor)
        (bind _player (message `/Game/Blueprints/I_Player.Get SE Player` OtherActor))
        (`/Game/Blueprints/BP_Player.Catch Souls` _player (`self.Souls`))
        (`NiagaraFunctionLibrary.SpawnSystemAtLocation` "/Game/FX/Dead/NE_Dead_System.NE_Dead_System" (`self.K2_GetActorLocation`))
        (`self.K2_DestroyActor`)))))

(event `/Game/Blueprints/I_Target.OnTarget`
  (bind _returnvalue (`GameplayStatics.SpawnEmitterAtLocation` "/Game/FX/Particles/P_Fire.P_Fire" (`self.K2_GetActorLocation`)))
  (set `self.Target FX` _returnvalue))

(event `/Game/Blueprints/I_Target.OnLoseTarget`
  (`self.Delete Target FX`))

(fn `Delete Target FX`
  (bind _target_fx (`self.Target FX`))
  (`/Engine/EditorBlueprintResources/StandardMacros.IsValid` _target_fx
    (:`Is Valid`
      (`ActorComponent.K2_DestroyComponent` _target_fx))))

(fn `Spawn Souls FX Attached`
  (params (Target :type "Actor Object Reference"))
  (bind _returnvalue (`NiagaraFunctionLibrary.SpawnSystemAttached` "/Game/FX/Souls/NE_Souls_System.NE_Souls_System" (`Actor.RootComponent` Target) "None" (0.0 0.0 0.0) (struct) "KeepRelativeOffset"))
  (`NiagaraComponent.SetVariableVec3` _returnvalue "User.NewVector" (`self.K2_GetActorLocation`)))

(fn `UserConstructionScript`)