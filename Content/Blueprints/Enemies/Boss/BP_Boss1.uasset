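; BP_Boss1 is a boss enemy Blueprint that triggers its melee attack through the Gameplay Ability System.
; The MelleAttack event activates the GA_BOSS_HIT1 ability on its AbilitySystemComponent.
; Tick calls the parent and prints the current stamina every frame as debug output.
; InAttack and InStamina are stubs that always return false.
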(event `self.ReceiveTick`
  (params (DeltaSeconds :type "Float (single-precision)"))
  (`parent.ReceiveTick` DeltaSeconds)
  (`KismetSystemLibrary.PrintString` (`KismetStringLibrary.Conv_DoubleToString` (`self.GetStamina`))))

(event `/Game/Blueprints/I_Melle.MelleAttack`
  (params (DistanceToPlayer :type "Float (single-precision)"))
  (`AbilitySystemComponent.TryActivateAbilityByClass` (`self.AbilitySystemComponent`) "/Game/Abilities/Enemies/BOSS/GA_BOSS_HIT1.GA_BOSS_HIT1_C" true))

(fn `InAttack`
  (returns (InAttack :type Boolean))
  (return false))

(fn `InStamina`
  (returns (InStamina :type Boolean))
  (return false))

(fn `UserConstructionScript`
  (`parent.UserConstructionScript`))