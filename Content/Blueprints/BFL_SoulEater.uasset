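; BFL_SoulEater is a Blueprint function library of shortcut getters for the game's SoulEater classes.
; Each helper casts a pawn's controller, an actor, the game instance or player controller 0 to its project class, returning early if the cast fails.
; InMainMenu builds on the game instance getter to expose its main menu flag.
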(fn `Get SE Character Base from Actor`
  (params (Actor :type "Actor Object Reference"))
  (returns (Character :type "/Game/Blueprints/BP_CharacterBase Object Reference"))
  (bind _asbp_character_base (cast `/Game/Blueprints/BP_CharacterBase` Actor))
  (return _asbp_character_base))

(fn `Get SE Game Instance`
  (returns (`AsSEGame Instance` :type "/Game/Blueprints/SEGameInstance Object Reference"))
  (bind _assegame_instance (cast `/Game/Blueprints/SEGameInstance` (`GameplayStatics.GetGameInstance` null)))
  (return _assegame_instance))

(fn `Get SE Pawn Controller`
  (params (Pawn :type "Pawn Object Reference"))
  (returns (`AsBP Player Controller` :type "/Game/Blueprints/BP_PlayerController Object Reference"))
  (bind _asbp_player_controller (cast `/Game/Blueprints/BP_PlayerController` (`Pawn.GetController` Pawn)))
  (return _asbp_player_controller))

(fn `Get SE Player Controller`
  (params (WorldContextObject :type "Object Object Reference"))
  (returns (`AsBP Player Controller` :type "/Game/Blueprints/BP_PlayerController Object Reference"))
  (bind _asbp_player_controller (cast `/Game/Blueprints/BP_PlayerController` (`GameplayStatics.GetPlayerController` WorldContextObject)))
  (return _asbp_player_controller))

(fn `In Main Menu`
  (returns (NewParam :type Boolean))
  (return (`/Game/Blueprints/SEGameInstance.In Main Menu` (`self.Get SE Game Instance` null))))