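; BP_Fire is a fire actor that registers itself with the player controller as the new fire when the player pawn touches it.
; Its sphere overlap calls SetNewFire, plays a fireball-cast sound, spawns an explosion emitter at the actor and prints a debug "Hello".
; A DoOnce gate resets after a short delay to throttle repeat triggers.
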(event `self.Sphere.OnComponentBeginOverlap`
  (params (OverlappedComponent :type "PrimitiveComponent Object Reference") (OtherActor :type "Actor Object Reference") (OtherComp :type "PrimitiveComponent Object Reference") (OtherBodyIndex :type Integer) (bFromSweep :type Boolean) (SweepResult :type "HitResult Structure (by ref)"))
  (if (== OtherActor (`GameplayStatics.GetPlayerPawn` 0))
    (`/Engine/EditorBlueprintResources/StandardMacros.DoOnce` false :!label _label
      (:`Completed`
        (`|ExecutionSequence`
          (:`then_0`
            (`/Game/Blueprints/BP_PlayerController.Set New Fire` (`/Game/Blueprints/BFL_SoulEater.Get SE Player Controller` self) self)
            (`GameplayStatics.PlaySound2D` "/Game/Assets/Sounds/Abilities/A_Ability_FireballCast_Cue.A_Ability_FireballCast_Cue" 0.2 1.0 0.0 null null)
            (`GameplayStatics.SpawnEmitterAtLocation` "/Game/FX/Particles/P_Explosion.P_Explosion" (`self.K2_GetActorLocation`) (struct) (2.0 2.0 2.0))
            (`KismetSystemLibrary.PrintString` "Hello"))
          (:`then_1`
            (`KismetSystemLibrary.Delay` 3.0)
            (goto _label :!via `Reset`)))))))

(fn `UserConstructionScript`)